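; Player controller that gives the controlled pawn basic movement, look and jump controls.
; Forward and right axis inputs move the pawn along the camera manager's forward and right vectors, so movement is camera-relative.
; Look axes feed pitch and yaw input on the controller, and the Jump action calls Jump when the pawn is a Character.
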(event EventBeginPlay)

(event EventTick
  (params (DeltaSeconds :type Float%20%28single-precision%29))
  ;[1 1 1] Basic Control
)

(event Input|ActionEvents|InputActionJump
  (params (Key :type Key%20Structure :default "None"))
  ;[1 1 1] Basic Control
  (:Pressed
    (bind _ascharacter (Utilities|Casting|CastToCharacter (Pawn|GetControlledPawn)))
    (Character|Jump _ascharacter)))

(event Input|AxisEvents|InputAxisMoveForward
  (params (AxisValue :type Float%20%28single-precision%29))
  ;[1 1 1] Basic Control
  (Pawn|Input|AddMovementInput (Pawn|GetControlledPawn) (Math|Vector|GetForwardVector (Camera|GetCameraRotation (Game|GetPlayerCameraManager 0))) AxisValue false))

(event Input|AxisEvents|InputAxisMoveRight
  (params (AxisValue :type Float%20%28single-precision%29))
  ;[1 1 1] Basic Control
  (Pawn|Input|AddMovementInput (Pawn|GetControlledPawn) (Math|Vector|GetRightVector (Camera|GetCameraRotation (Game|GetPlayerCameraManager 0))) AxisValue false))

(event Input|AxisEvents|InputAxisLookUp
  (params (AxisValue :type Float%20%28single-precision%29))
  ;[1 1 1] Basic Control
  (Class|PlayerController|AddPitchInput AxisValue))

(event Input|AxisEvents|InputAxisLookRight
  (params (AxisValue :type Float%20%28single-precision%29))
  ;[1 1 1] Basic Control
  (Class|PlayerController|AddYawInput AxisValue))

(fn ConstructionScript)