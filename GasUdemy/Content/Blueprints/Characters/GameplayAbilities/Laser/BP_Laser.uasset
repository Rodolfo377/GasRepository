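; BP_Laser is a laser beam actor for gameplay abilities whose skeletal mesh stretches to a detected end point.
; On BeginPlay it records the beam's original length from the actor to the mesh's "end" socket.
; Each tick it writes the difference between the distance to LazerEndDetector and that length into ABP_Lazer's EndBoneOffset, moving the end bone along X.
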(event Collision|EventActorBeginOverlap
  (params (OtherActor :type Actor%20Object%20Reference)))

(event EventTick
  (params (DeltaSeconds :type Float%20%28single-precision%29))
  (bind _asabp_lazer (Utilities|Casting|CastToABP_Lazer (Components|SkeletalMesh|GetAnimInstance (Variables|Default|GetLazerMesh))))
  (Variables|/Game/Blueprints/Characters/GameplayAbilities/Laser/Lazer_Ability_Assets/ABP_Lazer.ABP_Lazer_C|SetEndBoneOffset _asabp_lazer (Math|Vector|MakeVector (- (Math|Vector|VectorLength (- (Transformation|GetWorldLocation (Variables|Default|GetLazerEndDetector)) (Transformation|GetActorLocation))) (Variables|Default|GetBeamOriginalLength)) 0.0 0.0)))

(event EventBeginPlay
  (Variables|Default|SetBeamOriginalLength (Math|Vector|VectorLength (- (Transformation|GetSocketLocation (Variables|Default|GetLazerMesh) "end") (Transformation|GetActorLocation)))))

(fn ConstructionScript)