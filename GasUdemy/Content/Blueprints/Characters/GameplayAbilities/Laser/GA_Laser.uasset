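; GA_Laser is a gameplay ability that fires a sustained laser from the player character.
; On activation it commits, plays a casting montage, then attaches a spawned BP_Laser to the mesh's Laser socket and switches to camera-controlled rotation.
; Damage gameplay events apply GE_Laser_Damage and push-stun targets away from the beam end, or end the ability once cost is unaffordable.
; Ending removes the draining cost effect, destroys the laser and restores rotation.
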(event Ability|EventActivateAbility
  (Ability|CommitAbility)
  (CallFunction|DoUICooldown)
  (|PlayMontageandWaitProxy "None" "/Game/Blueprints/Characters/Animation/AM_Shinbi_Laser_Casting.AM_Shinbi_Laser_Casting" 1.0 "None" true 1.0
    (:then
      (Utilities|FlowControl|Delay 0.3)
      (bind _characterbase (CallFunction|GetPlayerCharacterandController))
      (bind _spawnedactor (|SpawnActor :Class "/Game/Blueprints/Characters/GameplayAbilities/Laser/BP_Laser.BP_Laser_C" :Instigator _characterbase)
        (:then
          (bind _output_get (Variables|Default|SetLaserActor _spawnedactor))
          (Transformation|AttachComponentToComponent _output_get (Variables|/Script/Engine.Character|GetMesh _characterbase) "Laser" "SnapToTarget" "SnapToTarget" "KeepRelative" true)
          (Default|MakeCameraControlRotation _characterbase true)
          (bind _payload (Ability|Tasks|WaitGameplayEvent "(TagName=\"skill.laser.dealDamage\")" 0)
            (:EventReceived
              (bind _output (CallFunction|IsCostStillAvailable))
              (if _output
                (GameplayEffects|ApplyGameplayEffectToTarget (.TargetData (Utilities|Struct|BreakGameplayEventData _payload)) "/Game/Blueprints/Characters/GameplayAbilities/Laser/GE_Laser_Damage.GE_Laser_Damage_C" 1 1)
                (for _array_element (Ability|TargetData|GetActorsfromTargetData (.TargetData (Utilities|Struct|BreakGameplayEventData _payload)))
                  (bind _asbp_character_base (Utilities|Casting|CastToBP_CharacterBase _array_element))
                  (Default|PushCharacter _asbp_character_base (Math|Vector|Normalize (- (Transformation|GetActorLocation _asbp_character_base) (Transformation|GetWorldLocation (Variables|/Game/Blueprints/Characters/GameplayAbilities/Laser/BP_Laser.BP_Laser_C|GetLaserEndDetector (.AsBP%20Laser (Utilities|Casting|CastToBP_Laser (Variables|Default|GetLaserActor))))))) 5e+02 0.3 "/Game/Blueprints/Characters/Animation/AM_Shinbi_HitStun.AM_Shinbi_HitStun"))
                (else
                  (Ability|EndAbility))))))))))

(event Ability|EventOnEndAbility
  (params (bWasCancelled :type Boolean))
  (Ability|RemoveGameplayEffectFromOwnerWithAssetTags "(GameplayTags=((TagName=\"skill.laser.drainingCost\")))")
  (Actor|DestroyActor (Variables|Default|GetLaserActor))
  (bind _characterbase (CallFunction|GetPlayerCharacterandController))
  (Default|MakeCameraControlRotation _characterbase false))