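; Fire Blast gameplay ability that pulls surrounding characters toward the caster, then damages and blasts them back.
; It commits, starts the UI cooldown and plays a montage, whose completion or interruption ends the ability.
; The pull gameplay event runs an instant radius target actor, stores the target data and pulls those characters with a stun.
; The push event reuses that data for damage and knockback, taking every direction from the last pulled character's position.
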(event Ability|EventActivateAbility
  (bind _returnvalue (Ability|CommitAbility))
  (if _returnvalue
    (CallFunction|DoUICooldown)
    (|PlayMontageandWaitProxy "None" "/Game/Blueprints/Characters/Animation/AM_FireBlast_Shinbi.AM_FireBlast_Shinbi" 1.0 "None" true 1.0
      (:then
        (Ability|Tasks|WaitGameplayEvent "(TagName=\"skill.FireBlast.pull\")" 0
          (:then
            (Ability|Tasks|WaitGameplayEvent "(TagName=\"skill.FireBlast.push\")" 0
              (:EventReceived
                (GameplayEffects|ApplyGameplayEffectToTarget (Variables|Default|GetTargetDataHandle) "/Game/Blueprints/Characters/GameplayAbilities/FireBlast/GE_FireBlastDamage.GE_FireBlastDamage_C" 1 1)
                (for _array_element (Ability|TargetData|GetActorsfromTargetData (Variables|Default|GetTargetDataHandle))
                  (bind _asbp_character_base (Utilities|Casting|CastToBP_CharacterBase _array_element))
                  (Default|PushCharacter _asbp_character_base (* (Math|Vector|Normalize (- (Transformation|GetActorLocation (Ability|GetOwningActorfromActorInfo)) (Transformation|GetActorLocation (stale _asbp_character_base_2)))) -1.0) 2e+03 2.0)))))
          (:EventReceived
            (bind _data (|WaitTargetData :ConfirmationType "Instant" :Class "/Script/GasUdemy.GATargetActorAround" :Radius 6e+02 :ReticleClass 0)
              (:ValidData
                (Variables|Default|SetTargetDataHandle _data)
                (for _array_element_2 (Ability|TargetData|GetActorsfromTargetData _data)
                  (bind _asbp_character_base_2 (Utilities|Casting|CastToBP_CharacterBase _array_element_2))
                  (Default|PushCharacter _asbp_character_base_2 (Math|Vector|Normalize (- (Transformation|GetActorLocation (Ability|GetOwningActorfromActorInfo)) (Transformation|GetActorLocation _asbp_character_base_2))) 1.5e+03 3.0)))))))
      (:OnCompleted
        (Ability|EndAbility :!label _label))
      (:OnBlendOut
        (goto _label))
      (:OnInterrupted
        (goto _label))
      (:OnCancelled
        (goto _label)))))

(event Ability|EventOnEndAbility
  (params (bWasCancelled :type Boolean)))